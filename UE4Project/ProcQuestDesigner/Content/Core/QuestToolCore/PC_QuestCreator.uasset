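; Player controller for the quest creator tool, setting up its main UI and handling global hotkeys.
; On BeginPlay it creates the WI_QuestDesignMain widget, shows the cursor and sets Game and UI input focused on it.
; F toggles fullscreen through GM_QuestTool.
; Escape and P both toggle the quit menu, reaching the QuestDesignWidget through a message call on the game mode rather than a stored widget reference.
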(event EventBeginPlay
  (bind _self self)
  ;[0 1 1] Create the main tool widget
  (bind _returnvalue (UserInterface|CreateWidget "/Game/Core/Widgets/MainScreen/WI_QuestDesignMain.WI_QuestDesignMain_C" _self))
  (UserInterface|Viewport|AddtoViewport _returnvalue 0)
  (Input|SetInputModeGameandUI _self _returnvalue "DoNotLock" false)
  (Variables|Default|SetbShowMouseCursor _self true))

(event Input|KeyboardEvents|Escape
  (params (Key :type Key%20Structure :default "None"))
  ;[0 1 1] On pressing escape open the exit menu
  (:Pressed
    (bind _questdesignwidget (Class|INQuestGamemode|GetQuestDesignMain(Message) (Game|GetGameMode)))
    (Class|INQuestDesignMain|ToggleQuitMenu(Message) _questdesignwidget)))

(event Input|KeyboardEvents|P
  (params (Key :type Key%20Structure :default "None"))
  ;[0 1 1] On pressing escape open the exit menu
  (:Pressed
    (bind _questdesignwidget (Class|INQuestGamemode|GetQuestDesignMain(Message) (Game|GetGameMode)))
    (Class|INQuestDesignMain|ToggleQuitMenu(Message) _questdesignwidget)))

(event Input|KeyboardEvents|F
  (params (Key :type Key%20Structure :default "None"))
  (:Pressed
    (bind _asgm_quest_tool (Utilities|Casting|CastToGM_QuestTool (Game|GetGameMode)))
    (Default|ToggleFullscreen _asgm_quest_tool)))

(fn ConstructionScript)